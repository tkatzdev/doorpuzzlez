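; Double door Blueprint that swings its left and right leaves open or closed when a character walks into a trigger.
; Separate Open and Close overlap components each filter the overlapping actor by checking whether its display name contains "character".
; Each trigger plays two timelines, one per leaf, to drive relative yaw.
; The timelines use Play without reversing or restarting, so finished ones do not replay on later overlaps.
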(event OnComponentBeginOverlap(close)
  (params (OverlappedComponent :type Primitive%20Component%20Object%20Reference) (OtherActor :type Actor%20Object%20Reference) (OtherComp :type Primitive%20Component%20Object%20Reference) (OtherBodyIndex :type Integer) (bFromSweep :type Boolean) (SweepResult :type Hit%20Result%20Structure%20%28by%20ref%29))
  (if (Utilities|String|Contains (Utilities|GetDisplayName OtherActor) "character")
    (Utilities|FlowControl|Sequence
      (:then_0
        (bind _dooropen (Timeline|close1 Play)
          (:Update
            (Transformation|SetRelativeRotation (Variables|Default|GetProtoDoorLeft) (Math|Rotator|MakeRotator 0.0 0.0 _dooropen) false false))))
      (:then_1
        (bind _dooropen_2 (Timeline|close2 Play)
          (:Update
            (Transformation|SetRelativeRotation (Variables|Default|Getrightdoor) (Math|Rotator|MakeRotator 0.0 0.0 _dooropen_2) false false)))))))

(event OnComponentBeginOverlap(open)
  (params (OverlappedComponent :type Primitive%20Component%20Object%20Reference) (OtherActor :type Actor%20Object%20Reference) (OtherComp :type Primitive%20Component%20Object%20Reference) (OtherBodyIndex :type Integer) (bFromSweep :type Boolean) (SweepResult :type Hit%20Result%20Structure%20%28by%20ref%29))
  ;[1 1 1] open door
  (if (Utilities|String|Contains (Utilities|GetDisplayName OtherActor) "character")
    (Utilities|FlowControl|Sequence
      (:then_0
        (bind _dooropen (Timeline|open1 Play)
          (:Update
            (Transformation|SetRelativeRotation (Variables|Default|GetProtoDoorLeft) (Math|Rotator|MakeRotator 0.0 0.0 _dooropen) false false))))
      (:then_1
        (bind _dooropen_2 (Timeline|open2 Play)
          (:Update
            (Transformation|SetRelativeRotation (Variables|Default|Getrightdoor) (Math|Rotator|MakeRotator 0.0 0.0 _dooropen_2) false false)))))))

(fn ConstructionScript)